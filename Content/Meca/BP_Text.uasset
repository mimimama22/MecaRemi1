(event `self.ReceiveBeginPlay`
  (`KismetSystemLibrary.K2_SetTimerDelegate` (`|CreateDelegate` :!event `TestPrefixX`) 0.5 true)
  (`KismetSystemLibrary.K2_SetTimerDelegate` (`|CreateDelegate` :!event `TextPrefixY`) 0.5 true))

(event `TestPrefixX`
  (bind _returnvalue (`self.K2_GetActorLocation`))
  (bind _returnvalue_2 (`self.K2_GetActorLocation`))
  (bind _refprefix_x (`self.RefPrefix_X`))
  (switch `/Game/Meca/EObjet` (`self.EObject`)
    (:`NewEnumerator0`
      (bind _outhit (`KismetSystemLibrary.LineTraceSingleForObjects` :`Start` _returnvalue :`End` (+ _returnvalue (-100.0 0.0 0.0)) :`ObjectTypes` (`|MakeArray` "ObjectTypeQuery2" :!type "EObjectTypeQuery Enum") :`DrawDebugType` "ForDuration"))
      (bind (_bblockinghit _binitialoverlap _time _distance _location _impactpoint _normal _impactnormal _physmat _hitactor) (`GameplayStatics.BreakHitResult` _outhit))
      (if _bblockinghit
        (bind _asbp_text (cast `/Game/Meca/BP_Text` _hitactor))
        (`KismetSystemLibrary.PrintText` (`|FormatText` "{A} : {B}" _asbp_text _refprefix_x))
        (if (not (== _asbp_text _refprefix_x))
          (`self.resetFunctionX`))
        (bind _output_get (set `self.RefPrefix_X` _asbp_text))
        (if (`/Game/Meca/BP_Text.IsPrefix` _output_get)
          (bind _outhit_2 (`KismetSystemLibrary.LineTraceSingleForObjects` :`Start` _returnvalue_2 :`End` (+ _returnvalue_2 (100.0 0.0 0.0)) :`ObjectTypes` (`|MakeArray` "ObjectTypeQuery2" :!type "EObjectTypeQuery Enum") :`DrawDebugType` "ForDuration"))
          (bind (_bblockinghit_2 _binitialoverlap_2 _time_2 _distance_2 _location_2 _impactpoint_2 _normal_2 _impactnormal_2 _physmat_2 _hitactor_2) (`GameplayStatics.BreakHitResult` _outhit_2))
          (if _bblockinghit_2
            (bind _asbp_text_2 (cast `/Game/Meca/BP_Text` _hitactor_2))
            (if (not (== _asbp_text_2 (`self.RefSufix_X`)))
              (`self.resetFunctionX`))
            (bind _output_get_2 (set `self.RefSufix_X` _asbp_text_2))
            (if (`/Game/Meca/BP_Text.IsSufix` _output_get_2)
              (`self.SetFonctionX`)
              (set `self.IsActive_X` true))
            (else
              (`self.resetFunctionX`))))
        (else
          (`self.resetFunctionX`))))))

(event `TextPrefixY`
  (bind _returnvalue (`self.K2_GetActorLocation`))
  (bind _returnvalue_2 (`self.K2_GetActorLocation`))
  (switch `/Game/Meca/EObjet` (`self.EObject`)
    (:`NewEnumerator0`
      (bind _outhit (`KismetSystemLibrary.LineTraceSingleForObjects` :`Start` _returnvalue_2 :`End` (+ _returnvalue_2 (0.0 -100.0 0.0)) :`ObjectTypes` (`|MakeArray` "ObjectTypeQuery2" :!type "EObjectTypeQuery Enum") :`DrawDebugType` "ForDuration"))
      (bind (_bblockinghit _binitialoverlap _time _distance _location _impactpoint _normal _impactnormal _physmat _hitactor) (`GameplayStatics.BreakHitResult` _outhit))
      (if _bblockinghit
        (bind _asbp_text (cast `/Game/Meca/BP_Text` _hitactor))
        (bind _output_get (set `self.RefPrefix_Y` _asbp_text))
        (if (`/Game/Meca/BP_Text.IsPrefix` _output_get)
          (bind _outhit_2 (`KismetSystemLibrary.LineTraceSingleForObjects` :`Start` _returnvalue :`End` (+ _returnvalue (0.0 100.0 0.0)) :`ObjectTypes` (`|MakeArray` "ObjectTypeQuery2" :!type "EObjectTypeQuery Enum") :`DrawDebugType` "ForDuration"))
          (bind (_bblockinghit_2 _binitialoverlap_2 _time_2 _distance_2 _location_2 _impactpoint_2 _normal_2 _impactnormal_2 _physmat_2 _hitactor_2) (`GameplayStatics.BreakHitResult` _outhit_2))
          (if _bblockinghit_2
            (bind _asbp_text_2 (cast `/Game/Meca/BP_Text` _hitactor_2))
            (bind _output_get_2 (set `self.RefSufix_Y` _asbp_text_2))
            (if (`/Game/Meca/BP_Text.IsSufix` _output_get_2)
              (`self.SetFunctionY`)
              (set `self.IsActive_Y` true))
            (else
              (`self.ResetFunctionY`))))
        (else
          (`self.ResetFunctionY`))))))

(event `SetFonctionX`
  (`KismetSystemLibrary.PrintString` "Set Function")
  (`|ExecutionSequence`
    (:`then_0`
      (`TextRenderComponent.SetTextRenderColor` (`self.TextRender`) (`|GetArrayItem` (`self.ColorActive`))))
    (:`then_1`
      (bind _refprefix_x (`self.RefPrefix_X`)
        (:`then`
          (`TextRenderComponent.SetTextRenderColor` (`/Game/Meca/BP_Text.TextRender` _refprefix_x) (`|GetArrayItem` (`self.ColorActive`) (`/Game/Meca/BP_Text.NColor` _refprefix_x)))
          (bind _refsufix_x (`self.RefSufix_X`)
            (:`then`
              (for _array_element (`self.RefObjet`)
                (if (== (`/Game/Meca/BP_Objet.ETypeObject` _array_element) (`KismetMathLibrary.Conv_ByteToInt` (`/Game/Meca/BP_Text.EObject` (`self.RefPrefix_X`))))
                  (`KismetSystemLibrary.PrintString` "Hello")
                  (switch `/Game/Meca/EObjet` (`/Game/Meca/BP_Text.EObject` _refsufix_x)
                    (:`NewEnumerator1`
                      (bind _cube (`/Game/Meca/BP_Objet.Cube` _array_element))
                      (`PrimitiveComponent.SetCollisionResponseToAllChannels` _cube "ECR_Block")
                      (`PrimitiveComponent.SetCollisionEnabled` _cube "QueryAndPhysics"))
                    (:`NewEnumerator2`
                      (`PrimitiveComponent.SetCollisionResponseToAllChannels` _cube "ECR_Overlap")
                      (`PrimitiveComponent.SetCollisionEnabled` _cube "QueryAndPhysics"))
                    (:`NewEnumerator3`
                      (`PrimitiveComponent.SetSimulatePhysics` _cube true)
                      (`PrimitiveComponent.SetCollisionEnabled` _cube "QueryAndPhysics")
                      (`PrimitiveComponent.SetCollisionResponseToAllChannels` _cube "ECR_Block"))))))
            (:`else`)))
        (:`else`)))
    (:`then_2`
      (bind _refsufix_x_2 (`self.RefSufix_X`)
        (:`then`
          (`TextRenderComponent.SetTextRenderColor` (`/Game/Meca/BP_Text.TextRender` _refsufix_x_2) (`|GetArrayItem` (`self.ColorActive`) (`/Game/Meca/BP_Text.NColor` _refsufix_x_2))))
        (:`else`)))))

(event `resetFunctionX`
  (`|ExecutionSequence`
    (:`then_0`
      (if (`self.IsActive_X`)
        (`TextRenderComponent.SetTextRenderColor` (`self.TextRender`) (`|GetArrayItem` (`self.ColorNotActive`)))
        (`KismetSystemLibrary.PrintString` "reset")
        (set `self.IsActive_X` false)))
    (:`then_1`
      (bind _refprefix_x (`self.RefPrefix_X`)
        (:`then`
          (`TextRenderComponent.SetTextRenderColor` (`/Game/Meca/BP_Text.TextRender` _refprefix_x) (`|GetArrayItem` (`self.ColorNotActive`) (`/Game/Meca/BP_Text.NColor` _refprefix_x)))
          (for _array_element (`self.RefObjet`)
            (bind _refprefix_x_2 (`self.RefPrefix_X`)
              (:`then`
                (if (== (`/Game/Meca/BP_Objet.ETypeObject` _array_element) (`KismetMathLibrary.Conv_ByteToInt` (`/Game/Meca/BP_Text.EObject` _refprefix_x_2)))
                  (bind _cube (`/Game/Meca/BP_Objet.Cube` _array_element))
                  (`PrimitiveComponent.SetSimulatePhysics` _cube false)
                  (`PrimitiveComponent.SetCollisionResponseToAllChannels` _cube "ECR_Ignore")))
              (:`else`))))
        (:`else`)))
    (:`then_2`
      (bind _refsufix_x (`self.RefSufix_X`)
        (:`then`
          (`TextRenderComponent.SetTextRenderColor` (`/Game/Meca/BP_Text.TextRender` _refsufix_x) (`|GetArrayItem` (`self.ColorNotActive`) (`/Game/Meca/BP_Text.NColor` _refsufix_x)))
          (set `self.RefSufix_X` null))
        (:`else`)))))

(event `SetFunctionY`
  (`KismetSystemLibrary.PrintString` "Set Function")
  (`|ExecutionSequence`
    (:`then_0`
      (`TextRenderComponent.SetTextRenderColor` (`self.TextRender`) (`|GetArrayItem` (`self.ColorActive`))))
    (:`then_1`
      (bind _refprefix_y (`self.RefPrefix_Y`)
        (:`then`
          (`TextRenderComponent.SetTextRenderColor` (`/Game/Meca/BP_Text.TextRender` _refprefix_y) (`|GetArrayItem` (`self.ColorActive`) (`/Game/Meca/BP_Text.NColor` _refprefix_y))))
        (:`else`)))
    (:`then_2`
      (bind _refsufix_y (`self.RefSufix_Y`)
        (:`then`
          (`TextRenderComponent.SetTextRenderColor` (`/Game/Meca/BP_Text.TextRender` _refsufix_y) (`|GetArrayItem` (`self.ColorActive`) (`/Game/Meca/BP_Text.NColor` _refsufix_y))))
        (:`else`)))))

(event `ResetFunctionY`
  (`|ExecutionSequence`
    (:`then_0`
      (if (`self.IsActive_Y`)
        (`TextRenderComponent.SetTextRenderColor` (`self.TextRender`) (`|GetArrayItem` (`self.ColorNotActive`)))
        (`KismetSystemLibrary.PrintString` "reset")
        (set `self.IsActive_Y` false)))
    (:`then_1`
      (bind _refprefix_y (`self.RefPrefix_Y`)
        (:`then`
          (`TextRenderComponent.SetTextRenderColor` (`/Game/Meca/BP_Text.TextRender` _refprefix_y) (`|GetArrayItem` (`self.ColorNotActive`) (`/Game/Meca/BP_Text.NColor` _refprefix_y)))
          (set `self.RefPrefix_Y` null))
        (:`else`)))
    (:`then_2`
      (bind _refsufix_y (`self.RefSufix_Y`)
        (:`then`
          (`TextRenderComponent.SetTextRenderColor` (`/Game/Meca/BP_Text.TextRender` _refsufix_y) (`|GetArrayItem` (`self.ColorNotActive`) (`/Game/Meca/BP_Text.NColor` _refsufix_y)))
          (set `self.RefSufix_Y` null))
        (:`else`)))))

(fn `UserConstructionScript`
  (`TextRenderComponent.K2_SetText` (`self.TextRender`) (`KismetTextLibrary.Conv_StringToText` (`|GetEnumeratorNameAsString` (`self.EObject`))))
  (switch `/Game/Meca/EObjet` (`self.EObject`)
    (:`NewEnumerator0`
      (`TextRenderComponent.SetTextRenderColor` (`self.TextRender`) (`|GetArrayItem` (`self.ColorNotActive`)))
      (set `self.NColor` 0))
    (:`NewEnumerator1`
      (set `self.IsSufix` true)
      (`TextRenderComponent.SetTextRenderColor` (`self.TextRender`) (`|GetArrayItem` (`self.ColorNotActive`) 1))
      (set `self.NColor` 1))
    (:`NewEnumerator2`
      (set `self.IsSufix` true)
      (`TextRenderComponent.SetTextRenderColor` (`self.TextRender`) (`|GetArrayItem` (`self.ColorNotActive`) 2))
      (set `self.NColor` 2))
    (:`NewEnumerator3`
      (set `self.IsSufix` true)
      (`TextRenderComponent.SetTextRenderColor` (`self.TextRender`) (`|GetArrayItem` (`self.ColorNotActive`) 3))
      (set `self.NColor` 3))
    (:`NewEnumerator4`
      (set `self.IsPrefix` true)
      (set `self.IsSufix` true)
      (`TextRenderComponent.SetTextRenderColor` (`self.TextRender`) (`|GetArrayItem` (`self.ColorNotActive`) 4))
      (set `self.NColor` 4))
    (:`NewEnumerator5`
      (set `self.IsPrefix` true)
      (set `self.IsSufix` true)
      (`TextRenderComponent.SetTextRenderColor` (`self.TextRender`) (`|GetArrayItem` (`self.ColorNotActive`) 5))
      (set `self.NColor` 5))
    (:`NewEnumerator6`
      (set `self.IsPrefix` true)
      (set `self.IsSufix` true)
      (`TextRenderComponent.SetTextRenderColor` (`self.TextRender`) (`|GetArrayItem` (`self.ColorNotActive`) 6))
      (set `self.NColor` 6))))